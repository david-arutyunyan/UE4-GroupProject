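; AI enemy that senses the player, selects animations and fires projectiles.
; Perception updates for PC_Player write sight status and the player reference to the Blackboard, with a debug print.
; AnimationStateMachine picks idle, walking or running animations, normal or aimed, from movement flags.
; Shoot checks ammo and reload state, spawns a weapon-dependent bullet at a yaw-rotated offset, then decrements ammo.
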(event OnTargetPerceptionUpdated(AIPerception)
  (params (Actor :type Actor%20Object%20Reference) (Stimulus :type AI%20Stimulus%20Structure))
  (bind _bsuccessfullysensed (Utilities|Struct|BreakAIStimulus Stimulus))
  (bind _aspc_player (Utilities|Casting|CastToPC_Player Actor))
  (AI|Components|Blackboard|SetValueasBool (AI|GetBlackboard self) (Utilities|Name|MakeLiteralName "IsSeePawn") _bsuccessfullysensed)
  (AI|Components|Blackboard|SetValueasObject (AI|GetBlackboard self) (Utilities|Name|MakeLiteralName "Player") _aspc_player)
  (Development|PrintString (Utilities|String|ToString(Boolean) _bsuccessfullysensed)))

(event EventBeginPlay)

(fn ConstructionScript)

(fn AnimationStateMachine
  (if (Variables|Movement|GetIsMoving)
    (if (Variables|Movement|GetIsSprinting)
      (Variables|Animations|SetAS_Normal "NewEnumerator2")
      (Variables|Default|SetAS_Aimed "NewEnumerator2")
      (else
        (Variables|Animations|SetAS_Normal "NewEnumerator1")
        (Variables|Default|SetAS_Aimed "NewEnumerator1")))
    (else
      (Variables|Animations|SetAS_Normal "NewEnumerator0")
      (Variables|Default|SetAS_Aimed "NewEnumerator0")))
  (return (select (Variables|Default|GetIsAiming) (Utilities|Select :Index (Variables|Default|GetAS_Aimed) :NewEnumerator0 (Variables|Animations|GetIdle_Aimed) :NewEnumerator1 (Variables|Animations|GetWalking_Aimed) :NewEnumerator2 (Variables|Animations|GetRunning_Aimed)) (Utilities|Select :Index (Variables|Animations|GetAS_Normal) :NewEnumerator0 (Variables|Animations|GetIdle) :NewEnumerator1 (Variables|Animations|GetWalking) :NewEnumerator2 (Variables|Animations|GetRunning)))))

(fn Shoot
  (bind _returnvalue (Transformation|GetActorLocation))
  (bind _returnvalue_2 (Transformation|GetActorRotation))
  (bind (_x _y _z) (Math|Vector|BreakVector _returnvalue))
  (bind _yaw (Math|Rotator|BreakRotator _returnvalue_2))
  (bind _returnvalue_3 (+ _yaw 4e+01))
  (if (and (> (Variables|Default|GetCurrentBullets) 0.0) (not (Variables|Default|GetIsReloading)))
    (LocalVariables|SetyOffset (* (Math|Trig|Sin(Degrees) _returnvalue_3) 9e+01))
    (LocalVariables|SetxOffset (* (Math|Trig|Cos(Degrees) _returnvalue_3) 9e+01))
    (if (Variables|Default|GetIsWeapon2)
      (Game|SpawnActorfromClass "/Game/MyContent/Blueprints/Bullet.Bullet_C" (Math|Transform|MakeTransform (Math|Vector|MakeVector (+ _x (LocalVariables|GetxOffset)) (+ _y (LocalVariables|GetyOffset)) _z) (Transformation|GetActorRotation) "0.100000,0.100000,0.100000") "Undefined" 0 0)
      (else
        (Game|SpawnActorfromClass "/Game/MyContent/Blueprints/Bullet_2.Bullet_2_C" (Math|Transform|MakeTransform (Math|Vector|MakeVector (+ _x (LocalVariables|GetxOffset)) (+ _y (LocalVariables|GetyOffset)) _z) (Transformation|GetActorRotation) "0.100000,0.100000,0.100000") "Undefined" 0 0)))
    (Variables|Default|SetCurrentBullets (- (Variables|Default|GetCurrentBullets) 1.0))))