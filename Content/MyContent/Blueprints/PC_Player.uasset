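; Player character with flipbook sprite animation, camera-relative movement, stamina-limited sprint, shooting and timed reload.
; Movement input updates the flipbook from moving, sprinting and aiming state; shots spawn one of two bullet classes at a yaw-based offset, chosen by holding LeftCtrl.
; Tick manages stamina and, on death, spawns a replacement possessed by player controller 1.
; Bonus overlaps refill health, stamina and ammo; the cursor-aim rotation is never called.
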(event OnComponentBeginOverlap(CapsuleComponent)
  (params (OverlappedComponent :type Primitive%20Component%20Object%20Reference) (OtherActor :type Actor%20Object%20Reference) (OtherComp :type Primitive%20Component%20Object%20Reference) (OtherBodyIndex :type Integer) (bFromSweep :type Boolean) (SweepResult :type Hit%20Result%20Structure%20%28by%20ref%29))
  (bind _asbonus (Utilities|Casting|CastToBonus OtherActor))
  (Actor|DestroyActor _asbonus)
  (Variables|Default|SetCurrentHealth (Variables|Default|GetMaxHealth))
  (Variables|Movement|SetStamina (Variables|Movement|GetMaxStamina))
  (Variables|Default|SetCurrentBullets (Variables|Default|GetMaxBullets)))

(event EventBeginPlay
  (Variables|Default|SetCurrentHealth (Variables|Default|GetMaxHealth))
  (Variables|Movement|SetStamina (Variables|Movement|GetMaxStamina))
  (bind _returnvalue (UserInterface|CreateWidget "/Game/MyContent/Blueprints/HUD.HUD_C" (Game|GetPlayerController 0)))
  (UserInterface|Viewport|AddtoViewport _returnvalue 0))

(event EventTick
  (params (DeltaSeconds :type Float%20%28single-precision%29))
  (if (<= (Variables|Default|GetCurrentHealth) 0.0)
    (Utilities|FlowControl|DoOnce false
      (:Completed
        (Actor|DestroyActor)
        (bind _returnvalue (Game|SpawnActorfromClass "PC_Player_C" (Math|Transform|MakeTransform "-1000.000000,300.000000,242.000671" "0, 0, 0" "1,1,1") "Undefined" 0 0))
        (Pawn|Possess (Game|GetPlayerController 1) _returnvalue))))
  (if (> (Variables|Movement|GetStamina) 0.5)
    _
    (else
      (Variables|Movement|SetCanSprint false)
      (Variables|Movement|SetCanSprint false)
      (CallFunction|StopSprint)))
  (if (and (Variables|Movement|GetIsMoving) (Variables|Movement|GetIsSprinting))
    (Variables|Movement|SetStamina (- (Variables|Movement|GetStamina) 0.5))
    (else
      (Variables|Movement|SetStamina (Math|Float|Clamp(Float) (+ (Variables|Movement|GetStamina) 0.1) 0.0 (Variables|Movement|GetMaxStamina)))
      (Utilities|FlowControl|Delay 1.0)
      (Variables|Movement|SetCanSprint true))))

(event Input|ActionEvents|InputActionShot
  (params (Key :type Key%20Structure :default "None"))
  (:Pressed
    (CallFunction|Shoot)))

(event Input|ActionEvents|InputActionReload
  (params (Key :type Key%20Structure :default "None"))
  (:Pressed
    (Variables|Default|SetIsReloading true)
    (Utilities|FlowControl|Delay 3.0)
    (Variables|Default|SetCurrentBullets 7.0)
    (Variables|Default|SetIsReloading false)))

(event Input|ActionEvents|InputActionAim
  (params (Key :type Key%20Structure :default "None"))
  (:Pressed
    (Variables|Default|SetIsAiming true)))

(event Input|KeyboardEvents|LeftCtrl
  (params (Key :type Key%20Structure :default "None"))
  (:Pressed
    (Variables|Default|SetIsWeapon2 true))
  (:Released
    (Variables|Default|SetIsWeapon2 false)))

(fn ConstructionScript)

(fn AnimationStateMachine
  (if (Variables|Movement|GetIsMoving)
    (if (Variables|Movement|GetIsSprinting)
      (Variables|Animations|SetAS_Normal "NewEnumerator2")
      (Variables|Default|SetAS_Aimed "NewEnumerator2")
      (else
        (Variables|Animations|SetAS_Normal "NewEnumerator1")
        (Variables|Default|SetAS_Aimed "NewEnumerator1")))
    (else
      (Variables|Animations|SetAS_Normal "NewEnumerator0")
      (Variables|Default|SetAS_Aimed "NewEnumerator0")))
  (return (select (Variables|Default|GetIsAiming) (Utilities|Select :Index (Variables|Default|GetAS_Aimed) :NewEnumerator0 (Variables|Animations|GetIdle_Aimed) :NewEnumerator1 (Variables|Animations|GetWalking_Aimed) :NewEnumerator2 (Variables|Animations|GetRunning_Aimed)) (Utilities|Select :Index (Variables|Animations|GetAS_Normal) :NewEnumerator0 (Variables|Animations|GetIdle) :NewEnumerator1 (Variables|Animations|GetWalking) :NewEnumerator2 (Variables|Animations|GetRunning)))))

(fn Shoot
  (bind _returnvalue (Transformation|GetActorLocation))
  (bind _returnvalue_2 (Transformation|GetActorRotation))
  (bind (_x _y _z) (Math|Vector|BreakVector _returnvalue))
  (bind _yaw (Math|Rotator|BreakRotator _returnvalue_2))
  (bind _returnvalue_3 (+ _yaw 4e+01))
  (if (and (> (Variables|Default|GetCurrentBullets) 0.0) (not (Variables|Default|GetIsReloading)))
    (LocalVariables|SetyOffset (* (Math|Trig|Sin(Degrees) _returnvalue_3) 9e+01))
    (LocalVariables|SetxOffset (* (Math|Trig|Cos(Degrees) _returnvalue_3) 9e+01))
    (if (Variables|Default|GetIsWeapon2)
      (Game|SpawnActorfromClass "/Game/MyContent/Blueprints/Bullet.Bullet_C" (Math|Transform|MakeTransform (Math|Vector|MakeVector (+ _x (LocalVariables|GetxOffset)) (+ _y (LocalVariables|GetyOffset)) _z) (Transformation|GetActorRotation) "0.100000,0.100000,0.100000") "Undefined" 0 0)
      (else
        (Game|SpawnActorfromClass "/Game/MyContent/Blueprints/Bullet_2.Bullet_2_C" (Math|Transform|MakeTransform (Math|Vector|MakeVector (+ _x (LocalVariables|GetxOffset)) (+ _y (LocalVariables|GetyOffset)) _z) (Transformation|GetActorRotation) "0.100000,0.100000,0.100000") "Undefined" 0 0)))
    (Variables|Default|SetCurrentBullets (- (Variables|Default|GetCurrentBullets) 1.0))))

(event Input|AxisEvents|InputAxisMoveForward
  (params (AxisValue :type Float%20%28single-precision%29))
  (Pawn|Input|AddMovementInput (Math|Vector|GetForwardVector (Math|Rotator|MakeRotator 0.0 0.0 (.Yaw (Math|Rotator|BreakRotator (Pawn|GetControlRotation :!class /Script/Engine.Pawn))))) AxisValue false)
  (CallFunction|UpdateAnimation))

(event Input|AxisEvents|InputAxisMoveRight
  (params (AxisValue :type Float%20%28single-precision%29))
  (Pawn|Input|AddMovementInput (Math|Vector|GetRightVector (Math|Rotator|MakeRotator 0.0 0.0 (.Yaw (Math|Rotator|BreakRotator (Pawn|GetControlRotation :!class /Script/Engine.Pawn))))) AxisValue false)
  (CallFunction|UpdateAnimation))

(event Custom|StopSprint
  (Variables|/Script/Engine.CharacterMovementComponent|SetMaxWalkSpeed (Variables|Character|GetCharacterMovement) (Variables|Movement|GetWalkSpeed))
  (Variables|Movement|SetIsSprinting false))

(event Input|ActionEvents|InputActionSprint
  (params (Key :type Key%20Structure :default "None"))
  (bind _charactermovement (Variables|Character|GetCharacterMovement))
  (:Pressed
    (if (Variables|Movement|GetCanSprint)
      (Variables|/Script/Engine.CharacterMovementComponent|SetMaxWalkSpeed _charactermovement (Variables|Movement|GetRunSpeed))
      (Variables|Movement|SetIsSprinting true)))
  (:Released
    (Variables|/Script/Engine.CharacterMovementComponent|SetMaxWalkSpeed _charactermovement (Variables|Movement|GetWalkSpeed))
    (Variables|Movement|SetIsSprinting false)))

(event Custom|Update%20Animation
  (bind _returnvalue (Transformation|GetVelocity))
  (bind _returnvalue_2 (Math|Vector|VectorLength _returnvalue))
  (Variables|Movement|SetCurrentSpeed _returnvalue_2)
  (Variables|Movement|SetIsMoving (> _returnvalue_2 0.0))
  (bind _flipbook (CallFunction|AnimationStateMachine))
  (Sprite|SetFlipbook (Variables|Default|GetSprite) _flipbook))