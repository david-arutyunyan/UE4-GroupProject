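; Player bullet actor that flies along its spawn yaw and damages AI enemies it hits.
; On BeginPlay it sets ProjectileMovement velocity from yaw and BulletSpeed, keeping travel horizontal.
; A Sphere hit on a BP_AIEnemy subtracts a fixed amount directly from its CurrentHealth.
; The hit does not destroy the bullet; Tick destroys it whenever its X velocity is exactly zero, regardless of Y.
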(event OnComponentHit(Sphere)
  (params (HitComponent :type Primitive%20Component%20Object%20Reference) (OtherActor :type Actor%20Object%20Reference) (OtherComp :type Primitive%20Component%20Object%20Reference) (NormalImpulse :type Vector :default "0, 0, 0") (Hit :type Hit%20Result%20Structure%20%28by%20ref%29))
  (bind _asbp_aienemy (Utilities|Casting|CastToBP_AIEnemy OtherActor))
  (Variables|/Game/MyContent/AI/BP_AIEnemy.BP_AIEnemy_C|SetCurrentHealth _asbp_aienemy (- (Variables|/Game/MyContent/AI/BP_AIEnemy.BP_AIEnemy_C|GetCurrentHealth _asbp_aienemy) 25.0)))

(event EventBeginPlay
  (bind _returnvalue (Transformation|GetActorRotation))
  (bind _bulletspeed (Variables|Default|GetBulletSpeed))
  (bind _yaw (Math|Rotator|BreakRotator _returnvalue))
  (Variables|/Script/Engine.MovementComponent|SetVelocity (Variables|Default|GetProjectileMovement) (Math|Vector|MakeVector (* (Math|Trig|Cos(Degrees) _yaw) _bulletspeed) (* (Math|Trig|Sin(Degrees) _yaw) _bulletspeed) 0.0)))

(event Collision|EventActorBeginOverlap
  (params (OtherActor :type Actor%20Object%20Reference)))

(event EventTick
  (params (DeltaSeconds :type Float%20%28single-precision%29))
  (if (== (.X (Math|Vector|BreakVector (Transformation|GetVelocity))) 0.0)
    (Actor|DestroyActor)))

(fn ConstructionScript)