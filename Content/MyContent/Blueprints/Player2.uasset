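; Player2 is a flipbook-sprite character with its own HUD_2 widget, gun and bonus pickups, shooting, reloading and stamina-limited sprinting.
; Overlapped guns set weapon flags and ammo, bonuses refill stats, and movement input picks the flipbook from the weapon flags.
; Shoot spawns PlayersBullet at a yaw-based offset, while Tick handles stamina and, at zero health, respawns by possessing a new Player2 at a random spawn.
; The cursor-aiming graph is never run.
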(event OnComponentBeginOverlap(CapsuleComponent)
  (params (OverlappedComponent :type Primitive%20Component%20Object%20Reference) (OtherActor :type Actor%20Object%20Reference) (OtherComp :type Primitive%20Component%20Object%20Reference) (OtherBodyIndex :type Integer) (bFromSweep :type Boolean) (SweepResult :type Hit%20Result%20Structure%20%28by%20ref%29))
  (bind _asbonus (Utilities|Casting|CastToBonus OtherActor)
    (:then
      (Actor|DestroyActor _asbonus)
      (CallFunction|Regeneration))
    (:CastFailed
      (bind _asgun_2 (Utilities|Casting|CastToGun2 OtherActor)
        (:then
          (Variables|Default|SetWithGun_2 true)
          (Variables|Default|SetWithGun_1 false)
          (Variables|Default|SetWithGun_3 false)
          (Variables|Default|SetMaxBullets 1e+02)
          (Variables|Default|SetCurrentBullets 1e+02)
          (Actor|DestroyActor _asgun_2))
        (:CastFailed
          (bind _asgun_3 (Utilities|Casting|CastToGun3 OtherActor)
            (:then
              (Variables|Default|SetWithGun_2 false)
              (Variables|Default|SetWithGun_1 false)
              (Variables|Default|SetWithGun_3 true)
              (Variables|Default|SetMaxBullets 1e+01)
              (Variables|Default|SetCurrentBullets 1e+01)
              (Actor|DestroyActor _asgun_3))
            (:CastFailed
              (bind _asgun_1 (Utilities|Casting|CastToGun1 OtherActor))
              (Variables|Default|SetWithGun_2 false)
              (Variables|Default|SetWithGun_1 true)
              (Variables|Default|SetWithGun_3 true)
              (Variables|Default|SetMaxBullets 7.0)
              (Variables|Default|SetCurrentBullets 7.0)
              (Actor|DestroyActor _asgun_1))))))))

(event EventBeginPlay
  (CallFunction|Regeneration)
  (Development|PrintString "Regenerated")
  (bind _asplayer_controller (Utilities|Casting|CastToPlayerController (Pawn|GetController)))
  (Development|PrintString "New widget")
  (bind _returnvalue (UserInterface|CreateWidget "/Game/MyContent/Blueprints/HUD_2.HUD_2_C" _asplayer_controller))
  (UserInterface|Viewport|AddtoPlayerScreen _returnvalue))

(event EventPossessed
  (params (NewController :type Controller%20Object%20Reference))
  (Development|PrintString "Possessed")
  (Utilities|IsValid (Pawn|GetControlledPawn NewController)
    (:Is%20Valid
      (bind _asplayer_controller (Utilities|Casting|CastToPlayerController (Pawn|GetController)))
      (Development|PrintString "New widget")
      (bind _returnvalue (UserInterface|CreateWidget "/Game/MyContent/Blueprints/HUD_2.HUD_2_C" _asplayer_controller))
      (UserInterface|Viewport|AddtoPlayerScreen _returnvalue))))

(event EventTick
  (params (DeltaSeconds :type Float%20%28single-precision%29))
  (if (<= (Variables|Default|GetCurrentHealth) 0.0)
    (Utilities|FlowControl|DoOnce false
      (:Completed
        (bind _returnvalue (Game|SpawnActorfromClass "Player2_C" (Math|Transform|MakeTransform (.OutItem (Utilities|Array|Random (Variables|Default|GetSpawns))) "0, 0, 0" "1,1,1") "Undefined" 0 0))
        (Development|PrintString "New Actor spawned")
        (bind _output_get (Variables|Default|SetContr (Pawn|GetController)))
        (Pawn|Possess _output_get _returnvalue)
        (Development|PrintString "New possess")
        (Development|PrintString "ALL WIDGETS REMOVED")
        (bind _asplayer_controller (Utilities|Casting|CastToPlayerController _output_get))
        (bind _returnvalue_2 (UserInterface|CreateWidget "/Game/MyContent/Blueprints/HUD_2.HUD_2_C" _asplayer_controller))
        (UserInterface|Viewport|AddtoPlayerScreen _returnvalue_2)
        (Actor|DestroyActor)
        (Development|PrintString "Actor destroyed")))
    (else
      (if (> (Variables|Movement|GetStamina) 0.5)
        _
        (else
          (Variables|Movement|SetCanSprint false)
          (Variables|Movement|SetCanSprint false)
          (CallFunction|StopSprint)))
      (if (and (Variables|Movement|GetIsMoving) (Variables|Movement|GetIsSprinting))
        (Variables|Movement|SetStamina (- (Variables|Movement|GetStamina) 0.5))
        (else
          (Variables|Movement|SetStamina (Math|Float|Clamp(Float) (+ (Variables|Movement|GetStamina) 0.1) 0.0 (Variables|Movement|GetMaxStamina)))
          (Utilities|FlowControl|Delay 1.0)
          (Variables|Movement|SetCanSprint true))))))

(event Input|ActionEvents|InputActionShot
  (params (Key :type Key%20Structure :default "None"))
  (:Pressed
    (CallFunction|Shoot)))

(event Input|ActionEvents|InputActionReload
  (params (Key :type Key%20Structure :default "None"))
  (:Pressed
    (Variables|Default|SetIsReloading true)
    (Utilities|FlowControl|Delay 3.0)
    (Variables|Default|SetCurrentBullets 7.0)
    (Variables|Default|SetIsReloading false)))

(event Input|ActionEvents|InputActionAim
  (params (Key :type Key%20Structure :default "None"))
  (:Pressed
    (Variables|Default|SetIsAiming true)))

(event Input|KeyboardEvents|LeftCtrl
  (params (Key :type Key%20Structure :default "None"))
  (:Pressed
    (Variables|Default|SetIsWeapon2 true))
  (:Released
    (Variables|Default|SetIsWeapon2 false)))

(fn ConstructionScript)

(fn AnimationStateMachine
  (if (Variables|Default|GetWithGun_1)
    (Variables|Animations|SetAS_Normal "NewEnumerator3")
    (elif (Variables|Default|GetWithGun_2)
      (Variables|Animations|SetAS_Normal "NewEnumerator4")
      (else
        (Variables|Animations|SetAS_Normal "NewEnumerator5"))))
  (return (Utilities|Select :Index (Variables|Animations|GetAS_Normal) :NewEnumerator3 (Variables|Animations|GetWithGun1) :NewEnumerator4 (Variables|Animations|GetWithGun2) :NewEnumerator5 (Variables|Animations|GetWithGun3))))

(fn Shoot
  (bind _returnvalue (Transformation|GetActorLocation))
  (bind _returnvalue_2 (Transformation|GetActorRotation))
  (bind (_x _y _z) (Math|Vector|BreakVector _returnvalue))
  (bind _yaw (Math|Rotator|BreakRotator _returnvalue_2))
  (bind _returnvalue_3 (+ _yaw 2e+01))
  (if (and (> (Variables|Default|GetCurrentBullets) 0.0) (not (Variables|Default|GetIsReloading)))
    (LocalVariables|SetyOffset (* (Math|Trig|Sin(Degrees) _returnvalue_3) 9e+01))
    (LocalVariables|SetxOffset (* (Math|Trig|Cos(Degrees) _returnvalue_3) 9e+01))
    (Game|SpawnActorfromClass "/Game/MyContent/Blueprints/PlayersBullet.PlayersBullet_C" (Math|Transform|MakeTransform (Math|Vector|MakeVector (+ _x (LocalVariables|GetxOffset)) (+ _y (LocalVariables|GetyOffset)) _z) (Transformation|GetActorRotation) "0.100000,0.100000,0.100000") "Undefined" 0 self 0)
    (Variables|Default|SetCurrentBullets (- (Variables|Default|GetCurrentBullets) 1.0))))

(fn Regeneration
  (Variables|Default|SetCurrentHealth (Variables|Default|GetMaxHealth))
  (Variables|Movement|SetStamina (Variables|Movement|GetMaxStamina))
  (Variables|Default|SetCurrentBullets (Variables|Default|GetMaxBullets)))

(event Input|AxisEvents|InputAxisMoveForward
  (params (AxisValue :type Float%20%28single-precision%29))
  (Pawn|Input|AddMovementInput (Math|Vector|GetForwardVector (Math|Rotator|MakeRotator 0.0 0.0 (.Yaw (Math|Rotator|BreakRotator (Pawn|GetControlRotation :!class /Script/Engine.Pawn))))) AxisValue false)
  (CallFunction|UpdateAnimation))

(event Input|AxisEvents|InputAxisMoveRight
  (params (AxisValue :type Float%20%28single-precision%29))
  (Pawn|Input|AddMovementInput (Math|Vector|GetRightVector (Math|Rotator|MakeRotator 0.0 0.0 (.Yaw (Math|Rotator|BreakRotator (Pawn|GetControlRotation :!class /Script/Engine.Pawn))))) AxisValue false)
  (CallFunction|UpdateAnimation))

(event Custom|StopSprint
  (Variables|/Script/Engine.CharacterMovementComponent|SetMaxWalkSpeed (Variables|Character|GetCharacterMovement) (Variables|Movement|GetWalkSpeed))
  (Variables|Movement|SetIsSprinting false))

(event Input|ActionEvents|InputActionSprint
  (params (Key :type Key%20Structure :default "None"))
  (bind _charactermovement (Variables|Character|GetCharacterMovement))
  (:Pressed
    (if (Variables|Movement|GetCanSprint)
      (Variables|/Script/Engine.CharacterMovementComponent|SetMaxWalkSpeed _charactermovement (Variables|Movement|GetRunSpeed))
      (Variables|Movement|SetIsSprinting true)))
  (:Released
    (Variables|/Script/Engine.CharacterMovementComponent|SetMaxWalkSpeed _charactermovement (Variables|Movement|GetWalkSpeed))
    (Variables|Movement|SetIsSprinting false)))

(event Custom|Update%20Animation
  (bind _returnvalue (Transformation|GetVelocity))
  (bind _returnvalue_2 (Math|Vector|VectorLength _returnvalue))
  (Variables|Movement|SetCurrentSpeed _returnvalue_2)
  (Variables|Movement|SetIsMoving (> _returnvalue_2 0.0))
  (bind _flipbook (CallFunction|AnimationStateMachine))
  (Sprite|SetFlipbook (Variables|Default|GetSprite) _flipbook))